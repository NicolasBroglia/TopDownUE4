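; BP_EnemyRanged is a ranged AI enemy that chases a target and shoots projectiles at the player.
; ChasePlayerRanged moves it within its attack-sphere radius, then OnAttackLogic spawns a projectile behind a short cooldown and turns it using a look-at rotation computed from actor scale, not location.
; Damage drains Health; death updates the game mode's enemy count for waves and destroys the actor.
; Attack and ShootAtPlayer are empty stubs.
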(event Custom|OnAttackLogic
  (params (Target :type Pawn%20Object%20Reference))
  ;[0.4678 1 0.9701] AtkLogic
  (bind _asthird_person_character (Utilities|Casting|CastToThirdPersonCharacter Target))
  (Utilities|FlowControl|Sequence
    (:then_0
      (if (Variables|Default|GetSpawnProyectile)
        (Game|SpawnActorfromClass "/Game/BP_ForEnemy.BP_ForEnemy_C" (Transformation|GetWorldTransform (Variables|Default|GetProyectile%20Spawn%20Location)) "Undefined" 0 0)
        (Variables|Default|SetSpawnProyectile false)
        (Utilities|FlowControl|Delay 0.7)
        (Variables|Default|SetSpawnProyectile true)))
    (:then_1
      (Transformation|SetActorRotation (Math|Rotator|MakeRotator (.roll (Math|Rotator|FindLookatRotation (Transformation|GetActorScale3D) (Transformation|GetActorLocation _asthird_person_character))) 0.0 (.yaw (Math|Rotator|FindLookatRotation (Transformation|GetActorScale3D) (Transformation|GetActorLocation _asthird_person_character))))))))

(event Custom|Death
  ;[1 0.384 0.4238] DeathLogic(EnemyWaves)
  (Variables|Default|SetIsDead true)
  (bind _asthird_person_game_mode (Utilities|Casting|CastToThirdPersonGameMode (Game|GetGameMode)))
  (Math|Integer|DecrementInt (Variables|/Game/ThirdPersonBP/Blueprints/ThirdPersonGameMode.ThirdPersonGameMode_C|GetEnemyAlive _asthird_person_game_mode)
    (:%20%20
      (Default|CheckEnemyLeft _asthird_person_game_mode)
      (Actor|DestroyActor))))

(event Custom|ChasePlayerRanged
  (params (Target :type Pawn%20Object%20Reference))
  (if (not (Variables|Default|GetIsDead))
    (AI|AIMoveTo self "0, 0, 0" Target (Variables|/Script/Engine.SphereComponent|GetSphereRadius (Variables|Default|GetAreaOfAtk)) false
      (:OnSuccess
        (CallFunction|OnAttackLogic Target)))))

(event Game|Damage|EventAnyDamage
  (params (Damage :type Float%20%28single-precision%29) (DamageType :type Damage%20Type%20Object%20Reference) (InstigatedBy :type Controller%20Object%20Reference) (DamageCauser :type Actor%20Object%20Reference))
  ;[0.3785 1 0.4775] Health
  (if (not (Variables|Default|GetIsDead))
    (Variables|Health|SetHealth (- (Variables|Health|GetHealth) Damage))
    (if (<= (Variables|Health|GetHealth) 0.0)
      (CallFunction|Death))))

(fn ConstructionScript)

(fn Attack)

(fn ShootatPlayer
  (params (Target :type Pawn%20Object%20Reference)))